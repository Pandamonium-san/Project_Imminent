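; Cave-ending trigger that freezes the monster, then sends it into a burst of extreme speed.
; When the player leaves the collision, it caches the monster's movement values, halts it and starts a timeout.
; The rush fires once, on timeout or when a per-tick camera trace hits this actor, with an impact sound and faster animation.
; A box spawned at the player's position restores normal speed when the monster overlaps it.
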(event OnComponentEndOverlap(CollisionComponent)
  (params (OverlappedComponent :type Primitive%20Component%20Object%20Reference) (OtherActor :type Actor%20Object%20Reference) (OtherComp :type Primitive%20Component%20Object%20Reference) (OtherBodyIndex :type Integer))
  ;[1 1 1] Activate tick on overlap and stop monster
  (if (== OtherActor (Variables|Default|GetPlayer))
    (Utilities|Casting|CastToCapsuleComponent OtherComp)
    (Utilities|FlowControl|DoOnce false
      (:Completed
        (Utilities|FlowControl|Delay 0.2)
        (bind _outactors (Actor|GetAllActorsOfClass "/Game/ImminentCPP/Blueprints/AI/Monster_BP.Monster_BP_C"))
        (Variables|Default|SetMonster (Utilities|Array|Get(acopy) _outactors))
        (Actor|Tick|SetActorTickEnabled (Variables|Default|GetMonster))
        (Pawn|Components|CharacterMovement|DisableMovement (Variables|/Script/Engine.Character|GetCharacterMovement (Variables|Default|GetMonster)))
        (Actor|Tick|SetActorTickEnabled true)
        (Variables|Default|SetMonsterWalkSpeed (Variables|/Script/Engine.CharacterMovementComponent|GetMaxWalkSpeed (Variables|/Script/Engine.Character|GetCharacterMovement (Variables|Default|GetMonster))))
        (Variables|Default|SetMonsterAcceleration (Class|CharacterMovementComponent|GetMaxAcceleration (Variables|/Script/Engine.Character|GetCharacterMovement (Variables|Default|GetMonster))))
        (Utilities|Time|SetTimerbyEvent (delegate Custom|DoRapid) (Variables|Default|GetTimeout))
        (Development|PrintText "rapid triggered")))))

(event Custom|OnComponentBeginOverlap_Event_0
  (params (OverlappedComponent :type Primitive%20Component%20Object%20Reference) (OtherActor :type Actor%20Object%20Reference) (OtherComp :type Primitive%20Component%20Object%20Reference) (OtherBodyIndex :type Integer) (bFromSweep :type Boolean) (SweepResult :type Hit%20Result%20Structure%20%28by%20ref%29))
  (bind _monster (Variables|Default|GetMonster))
  (bind _charactermovement (Variables|/Script/Engine.Character|GetCharacterMovement _monster))
  ;[1 1 1] Reset monster speed on box overlap
  (if (== OtherActor (Variables|Default|GetMonster))
    (bind _output_get (Variables|/Game/ImminentCPP/Blueprints/AI/Monster_BP.Monster_BP_C|SetMaxWalkSpeed _monster (Variables|Default|GetMonsterWalkSpeed)))
    (Variables|/Script/Engine.CharacterMovementComponent|SetMaxWalkSpeed _charactermovement _output_get)
    (Variables|/Script/Engine.CharacterMovementComponent|SetMaxAcceleration _charactermovement (Variables|Default|GetMonsterAcceleration))
    (Variables|/Script/Engine.SkeletalMeshComponent|SetGlobalAnimRateScale (Variables|/Script/Engine.Character|GetMesh _monster) 1.0)
    (Development|PrintText "end")
    (Collision|UnbindEventfromOnComponentBeginOverlap OverlappedComponent (delegate Custom|OnComponentBeginOverlap_Event_0))))

(event Custom|DoRapid
  (bind _monster (Variables|Default|GetMonster))
  (bind _charactermovement (Variables|/Script/Engine.Character|GetCharacterMovement _monster))
  ;[1 1 1] Line trace from player camera
  (Utilities|FlowControl|DoOnce false
    (:Completed
      ;[1 1 1] Create box collision
      (bind _returnvalue (AddComponent|AddBoxComponent false (Math|Transform|MakeTransform "0, 0, 0" "0, 0, 0" "5.000000,5.000000,5.000000")))
      (Collision|AssignOnComponentBeginOverlap _returnvalue (delegate Custom|OnComponentBeginOverlap_Event_0))
      (Transformation|SetWorldLocation _returnvalue (Transformation|GetActorLocation (Variables|Default|GetPlayer)) false false)
      (Collision|SetCollisionResponsetoChannel _returnvalue "ECC_WorldDynamic" "ECR_Overlap")
      ;[1 1 1] Increase monster speed
      (Audio|PlaySoundatLocation "/Game/ImminentContent/Audio/Metal_Impact_Sound_Effect_Cue.Metal_Impact_Sound_Effect_Cue" (Transformation|GetActorLocation _monster) "0, 0, 0" 1.0 1.0 0.0 "/Game/ImminentContent/Audio/Attenuation/Monster_Attenuation.Monster_attenuation")
      (Actor|Tick|SetActorTickEnabled _monster true)
      (bind _output_get (Variables|/Game/ImminentCPP/Blueprints/AI/Monster_BP.Monster_BP_C|SetMaxWalkSpeed _monster (Variables|Default|GetRapidWalkSpeed)))
      (Variables|/Script/Engine.CharacterMovementComponent|SetMaxWalkSpeed _charactermovement _output_get)
      (Variables|/Script/Engine.CharacterMovementComponent|SetMaxAcceleration _charactermovement 2e+05)
      (Pawn|Components|CharacterMovement|SetMovementMode _charactermovement "MOVE_Walking" 0)
      (Variables|/Script/Engine.SkeletalMeshComponent|SetGlobalAnimRateScale (Variables|/Script/Engine.Character|GetMesh _monster) 5.0)
      (Development|PrintText "speed triggered")
      (Actor|Tick|SetActorTickEnabled false))))

(event EventBeginPlay
  (Actor|Tick|SetActorTickEnabled false)
  (bind _asproject_imminent_character_bp (Utilities|Casting|CastToProject_ImminentCharacter_BP (Game|GetPlayerCharacter 0)))
  (Variables|Default|SetPlayer _asproject_imminent_character_bp))

(event EventTick
  (params (DeltaSeconds :type Float%20%28single-precision%29))
  (bind _player (Variables|Default|GetPlayer))
  (bind _monster (Variables|Default|GetMonster))
  (bind _firstpersoncameracomponent (Variables|/Script/Project_Imminent.Project_ImminentCharacter|GetFirstPersonCameraComponent _player))
  (bind _charactermovement (Variables|/Script/Engine.Character|GetCharacterMovement _monster))
  (bind _returnvalue (Transformation|GetWorldLocation _firstpersoncameracomponent))
  ;[1 1 1] Line trace from player camera
  (bind _outhit (Collision|LineTraceByChannel _returnvalue (+ _returnvalue (* (Math|Vector|GetForwardVector _firstpersoncameracomponent) 1e+04)) "TraceTypeQuery2" false (Utilities|Array|MakeArray _player) "None" false))
  (if (== (.HitActor (Collision|BreakHitResult _outhit)) self)
    (Utilities|FlowControl|DoOnce false
      (:Completed
        ;[1 1 1] Create box collision
        (bind _returnvalue_2 (AddComponent|AddBoxComponent false (Math|Transform|MakeTransform "0, 0, 0" "0, 0, 0" "5.000000,5.000000,5.000000")))
        (Collision|AssignOnComponentBeginOverlap _returnvalue_2 (delegate Custom|OnComponentBeginOverlap_Event_0))
        (Transformation|SetWorldLocation _returnvalue_2 (Transformation|GetActorLocation (Variables|Default|GetPlayer)) false false)
        (Collision|SetCollisionResponsetoChannel _returnvalue_2 "ECC_WorldDynamic" "ECR_Overlap")
        ;[1 1 1] Increase monster speed
        (Audio|PlaySoundatLocation "/Game/ImminentContent/Audio/Metal_Impact_Sound_Effect_Cue.Metal_Impact_Sound_Effect_Cue" (Transformation|GetActorLocation _monster) "0, 0, 0" 1.0 1.0 0.0 "/Game/ImminentContent/Audio/Attenuation/Monster_Attenuation.Monster_attenuation")
        (Actor|Tick|SetActorTickEnabled _monster true)
        (bind _output_get (Variables|/Game/ImminentCPP/Blueprints/AI/Monster_BP.Monster_BP_C|SetMaxWalkSpeed _monster (Variables|Default|GetRapidWalkSpeed)))
        (Variables|/Script/Engine.CharacterMovementComponent|SetMaxWalkSpeed _charactermovement _output_get)
        (Variables|/Script/Engine.CharacterMovementComponent|SetMaxAcceleration _charactermovement 2e+05)
        (Pawn|Components|CharacterMovement|SetMovementMode _charactermovement "MOVE_Walking" 0)
        (Variables|/Script/Engine.SkeletalMeshComponent|SetGlobalAnimRateScale (Variables|/Script/Engine.Character|GetMesh _monster) 5.0)
        (Development|PrintText "speed triggered")
        (Actor|Tick|SetActorTickEnabled false)))))

(fn ConstructionScript)