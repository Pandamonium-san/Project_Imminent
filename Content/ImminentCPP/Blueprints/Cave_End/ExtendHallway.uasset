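; ExtendHallway is a one-shot trigger in the cave ending that makes a hallway appear longer by rearranging the level around the player.
; On TriggerEvent it teleports HallwayParent to the world origin, then shifts RoomParent and the player along negative X by segment count times segment length.
; The matching offset keeps the player in place relative to the room, with movement paused during the teleports.
; It then clears UserInteractable.
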(event EventBeginPlay)

(event EventTick
  (params (DeltaSeconds :type Float%20%28single-precision%29)))

(event EventTriggerEvent
  (bind _returnvalue (Game|GetPlayerCharacter 0))
  (bind _hallwaysegments (Variables|Default|GetHallwaySegments))
  (bind _segmentlength (Variables|Default|GetSegmentLength))
  (bind _returnvalue_2 (* _hallwaysegments _segmentlength))
  (bind _charactermovement (Variables|/Script/Engine.Character|GetCharacterMovement _returnvalue))
  (bind _returnvalue_3 (* _returnvalue_2 -1.0))
  (bind _returnvalue_4 (Math|Vector|MakeVector _returnvalue_3 0.0 0.0))
  (Pawn|Components|CharacterMovement|DisableMovement _charactermovement)
  (Transformation|SetActorLocation (Variables|Default|GetHallwayParent) "0, 0, 0" false true)
  (Transformation|AddActorWorldOffset (Variables|Default|GetRoomParent) _returnvalue_4 false true)
  (Transformation|AddActorWorldOffset (Game|GetPlayerCharacter 0) _returnvalue_4 false true)
  (Pawn|Components|CharacterMovement|SetMovementMode _charactermovement "MOVE_Walking" 0)
  (Variables|Default|SetUserInteractable false))