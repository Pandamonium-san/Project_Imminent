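; Bridge lever actor that animates a lever mesh when its bridge trigger component is activated.
; Activation plays a timeline that drives the mesh's relative roll and deactivates the trigger component on each update.
; When the forward swing finishes, the lever waits briefly and reverses, with a Done flag stopping the Finished event from looping.
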(event OnComponentActivated(BridgeTrigger_BP)
  (params (bReset :type Boolean))
  (Variables|Default|Setdone false)
  (bind _newtrack_4 (Timeline|Rotatelever Play)
    (:Update
      (Transformation|SetRelativeRotation (Variables|Default|GetStaticMesh1) (Math|Rotator|MakeRotator _newtrack_4 0.0 0.0) false false)
      (Components|Activation|Deactivate (Variables|Default|GetBridgeTrigger_BP)))
    (:Finished
      (if (not (Variables|Default|Getdone))
        (Utilities|FlowControl|Delay 5.0)
        (Variables|Default|Setdone true)
        (Timeline|Rotatelever Reverse)))))

(event EventBeginPlay)

(event Collision|EventActorBeginOverlap
  (params (OtherActor :type Actor%20Object%20Reference)))

(fn ConstructionScript)