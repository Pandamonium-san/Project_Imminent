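; Bridge Blueprint that plays the sounds for a bridge in the bridge sequence when it activates or resets.
; Tick polls Active and IsResetting, each gating a do-once that re-arms when its flag clears.
; Each trigger plays BridgeMovingCue, then BridgeCue2 two seconds later.
; The graph holds no movement logic, and two leftover PlaySoundAtLocation calls are never executed.
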(event EventBeginPlay)

(event Collision|EventActorBeginOverlap
  (params (OtherActor :type Actor%20Object%20Reference)))

(event EventTick
  (params (DeltaSeconds :type Float%20%28single-precision%29))
  (bind _bridge_moving_cue (Variables|Default|Getbridge_moving_Cue))
  (bind _bridge_cue2 (Variables|Default|GetBridge_cue2))
  (Utilities|FlowControl|Sequence
    (:then_0
      (if (Variables|Default|GetbActive)
        (Utilities|FlowControl|DoOnce true :!label _label
          (:Completed
            (Audio|Components|Audio|Play _bridge_moving_cue 0.0)
            (Utilities|FlowControl|Delay 2.0)
            (Audio|Components|Audio|Play _bridge_cue2 0.0)))
        (else
          (goto _label Reset))))
    (:then_1
      (if (Variables|Default|GetbIsResetting)
        (Utilities|FlowControl|DoOnce true :!label _label_2
          (:Completed
            (Audio|Components|Audio|Play _bridge_moving_cue 0.0)
            (Utilities|FlowControl|Delay 2.0)
            (Audio|Components|Audio|Play _bridge_cue2 0.0)))
        (else
          (goto _label_2 Reset))))))

(fn ConstructionScript)