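; First-person player character that adds the HUD, movement feedback and death sequences, and hides the right arm at start.
; Tick drives distance-based, surface-specific footsteps, plus head bob and an FOV timeline while running.
; An overlap volume tracks items underfoot, releasing the grabbed item if stood upon, with bone matching for destructibles.
; Death selects jumpscare, electrocution or water-gate smash by index, then respawns at the checkpoint.
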(event OnComponentBeginOverlap(AntiStandOnItemCollision)
  (params (OverlappedComponent :type Primitive%20Component%20Object%20Reference) (OtherActor :type Actor%20Object%20Reference) (OtherComp :type Primitive%20Component%20Object%20Reference) (OtherBodyIndex :type Integer) (bFromSweep :type Boolean) (SweepResult :type Hit%20Result%20Structure%20%28by%20ref%29))
  ;[1 1 1] Track which items are stood upon
  (bind _returnvalue (Utilities|Array|Add (Variables|Default|GetItemsStoodOn) OtherComp))
  (Utilities|Array|SetArrayElem (Variables|Default|GetItemsStoodOnBodyIndex) _returnvalue OtherBodyIndex true))

(event OnComponentEndOverlap(AntiStandOnItemCollision)
  (params (OverlappedComponent :type Primitive%20Component%20Object%20Reference) (OtherActor :type Actor%20Object%20Reference) (OtherComp :type Primitive%20Component%20Object%20Reference) (OtherBodyIndex :type Integer))
  (bind _itemsstoodon (Variables|Default|GetItemsStoodOn))
  (bind _itemsstoodonbodyindex (Variables|Default|GetItemsStoodOnBodyIndex))
  ;[1 1 1] Track which items are stood upon
  (for _index (range 0 (Utilities|Array|Length (Variables|Default|GetItemsStoodOn)))
    (if (and (== (Utilities|Array|Get(acopy) _itemsstoodon _index) OtherComp) (== (Utilities|Array|Get(acopy) _itemsstoodonbodyindex _index) OtherBodyIndex))
      (Utilities|Array|RemoveIndex _itemsstoodonbodyindex _index)
      (Utilities|Array|RemoveIndex _itemsstoodon _index))))

(event Custom|Death
  (params (Index :type Integer))
  (switch int Index
    (:Default
      ;[1 1 1] Death_Jumpscare
      (Utilities|FlowControl|Delay 0.5 :!label _label)
      (Input|DisableInput (Game|Player|GetPlayerPawn 0) 0)
      (Variables|/Script/Engine.CameraComponent|SetPostProcessSettings (Variables|Default|GetFirstPersonCameraComponent) (Utilities|Struct|MakePostProcessSettings "(R=0.265000,G=0.185181,B=0.155798,A=1.000000)"))
      (Class|PlayerController|ClientPlayCameraShake (Game|GetPlayerController 0) "/Game/ImminentCPP/Blueprints/CameraShake_DeathShake.CameraShake_DeathShake_C" 5.0 "CameraLocal" "0, 0, 0")
      (Audio|PlaySound2D "/Game/ImminentContent/Audio/333832_nick121087_demonic-woman-scream_converted.333832_nick121087_demonic-woman-scream_converted" 3.0 5.0)
      (Rendering|SetVisibility (Variables|Default|GetJumpScareMonsterFace) true false)
      (Rendering|SetVisibility (Variables|Default|GetMonsterFaceLight) true false)
      (Utilities|FlowControl|Delay 1.0)
      (Variables|/Script/Engine.CameraComponent|SetPostProcessSettings (Variables|Default|GetFirstPersonCameraComponent) (Utilities|Struct|MakePostProcessSettings "(R=0.000000,G=0.000000,B=0.000000,A=1.000000)"))
      (Utilities|FlowControl|Delay 2.0)
      (Class|ProjectImminentCharacter|RespawnatCheckpoint)
      (Rendering|SetVisibility (Variables|Default|GetJumpScareMonsterFace) false false)
      (Rendering|SetVisibility (Variables|Default|GetMonsterFaceLight) false false)
      (Utilities|FlowControl|Delay 1.0)
      (Input|EnableInput (Game|Player|GetPlayerPawn 0) 0)
      (Variables|/Script/Engine.CameraComponent|SetbUsePawnControlRotation (Variables|Default|GetFirstPersonCameraComponent) true)
      (Pawn|Components|CharacterMovement|SetMovementMode (Variables|Character|GetCharacterMovement) "MOVE_Walking" 0)
      (Variables|/Script/Engine.CameraComponent|SetPostProcessSettings (Variables|Default|GetFirstPersonCameraComponent) (Utilities|Struct|MakePostProcessSettings "(R=1.000000,G=1.000000,B=1.000000,A=1.000000)")))
    (:0
      (goto _label))
    (:1
      ;[1 1 1] Death_Electricity
      (Input|DisableInput (Game|Player|GetPlayerPawn 0) 0)
      (Development|PrintText "electric death")
      (Class|PlayerController|ClientPlayCameraShake (Game|GetPlayerController 0) "/Game/ImminentCPP/Blueprints/CameraShake_Electrocution.CameraShake_Electrocution_C" 1.0 "CameraLocal" "0, 0, 0")
      (Utilities|FlowControl|Delay 3.0)
      (CallFunction|Respawn))
    (:2
      ;[1 1 1] Death_Watersmash
      (Input|DisableInput (Game|Player|GetPlayerPawn 0) 0)
      (Development|PrintText "gatesmash death")
      (Utilities|FlowControl|Delay 3.0)
      (CallFunction|Respawn))))

(event EventBeginPlay
  (bind _returnvalue (UserInterface|CreateWidget "/Game/ImminentCPP/Blueprints/GUI/HUD.HUD_C"))
  (bind _output_get (Variables|Default|SetHUD%20Reference _returnvalue))
  (UserInterface|Viewport|AddtoViewport _output_get 0)
  (Components|SkinnedMesh|HideBonebyName (Variables|Default|GetSkeletalMesh) "r_sk_root_shoulder" "PBO_None") ; Hides right arm at start
)

(event EventTick
  (params (DeltaSeconds :type Float%20%28single-precision%29))
  (bind _returnvalue (Transformation|GetVelocity))
  (bind _charactermovement (Variables|Character|GetCharacterMovement))
  (bind _returnvalue_2 (Math|Vector|VectorLength _returnvalue))
  (bind _movementmode (Variables|/Script/Engine.CharacterMovementComponent|GetMovementMode _charactermovement))
  (bind _returnvalue_3 (Utilities|Select :Index _movementmode :MOVE_None false :MOVE_Walking true :MOVE_NavWalking false :MOVE_Falling false :MOVE_Swimming false :MOVE_Flying false :MOVE_Custom false))
  (CallFunction|CheckStandingonGrabbedItem)
  (if (> _returnvalue_2 0.0)
    ;[1 1 1] Footstep sound
    (if _returnvalue_3
      (bind _output_get (Variables|Default|SetDistanceTravelled (+ (* DeltaSeconds _returnvalue_2) (stale _output_get))))
      (if (>= _output_get (Variables|Default|GetStepSize))
        (CallFunction|PlayFootstep)
        (else
          (if (Variables|Default|GetbRunning) :!label _label
            (if _returnvalue_3
              (Class|PlayerController|ClientPlayCameraShake (Game|GetPlayerController 0) "/Game/ImminentCPP/Blueprints/CameraShake_HeadBob.CameraShake_HeadBob_C" 1.0 "CameraLocal" "0, 0, 0")
              (bind _fov_track (Timeline|FoV_TimeLine Play)
                (:Update
                  (Camera|SetFieldOfView (Variables|Default|GetFirstPersonCameraComponent) _fov_track)))
              (else
                (Timeline|FoV_TimeLine Play)))
            (else
              (Timeline|FoV_TimeLine Reverse)))))
      (else
        (Variables|Default|SetDistanceTravelled (Variables|Default|GetStepSize))
        (goto _label)))
    (else
      (Variables|Default|SetbRunning false))))

(fn ConstructionScript)

(fn PlayFootstep
  (bind _returnvalue (Transformation|GetActorLocation))
  (bind (_outhit _returnvalue_2) (Collision|LineTraceByChannel (+ _returnvalue "0, 0,50.000000") (+ _returnvalue "0, 0,-170.000000") "TraceTypeQuery1" false 0 "None"))
  (if _returnvalue_2
    (Audio|PlaySoundatLocation (Utilities|Select :Index (Collision|GetSurfaceType _outhit) :SurfaceType_Default "/Game/ImminentContent/Audio/Footsteps/Footstep_concrete.Footstep_concrete" :SurfaceType1 "/Game/ImminentContent/Audio/Footsteps/Footstep_concrete.Footstep_concrete" :SurfaceType2 "/Game/ImminentContent/Audio/Footsteps/Footstep_wood.Footstep_wood" :SurfaceType3 "/Game/ImminentContent/Audio/Footsteps/Footstep_gravel.Footstep_gravel" :SurfaceType4 "/Game/ImminentContent/Audio/Footsteps/Footstep_water.Footstep_water") (.Location (Collision|BreakHitResult _outhit)))
    (Variables|Default|SetDistanceTravelled 0.0)))

(fn CheckStandingonGrabbedItem
  (bind _grabbedcomponent (Variables|Default|GetGrabbedComponent))
  (Utilities|IsValid _grabbedcomponent
    (:Is%20Valid
      (for (_array_element _array_index) (Variables|Default|GetItemsStoodOn)
        (if (== _array_element _grabbedcomponent)
          (bind _asdestructible_component (Utilities|Casting|CastToDestructibleComponent _array_element)
            (:then
              (Development|PrintText (Utilities|Text|ToText(Name) (Class|SkinnedMeshComponent|GetBoneName _asdestructible_component (Utilities|Array|Get(acopy) (Variables|Default|GetItemsStoodOnBodyIndex) _array_index))))
              (if (Utilities|Name|Equal(Name) (Class|SkinnedMeshComponent|GetBoneName _asdestructible_component (Utilities|Array|Get(acopy) (Variables|Default|GetItemsStoodOnBodyIndex) _array_index)) (Variables|Default|GetGrabbedBoneName))
                (Development|PrintText "same bone")
                (Class|ProjectImminentCharacter|Release :!label _label)))
            (:CastFailed
              (goto _label))))))))

(fn Respawn
  (Class|ProjectImminentCharacter|RespawnatCheckpoint)
  (Input|EnableInput (Game|Player|GetPlayerPawn 0) 0)
  (Variables|/Script/Engine.CameraComponent|SetbUsePawnControlRotation (Variables|Default|GetFirstPersonCameraComponent) true))