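; CloseToKill is a behavior tree decorator for the monster AI that gates a branch on distance to its followed target.
; It casts the owning controller to MonsterAIController_BP and measures between the controlled pawn and the TargetToFollow blackboard actor.
; Despite the name, the condition passes when that distance is at or beyond AcceptedDistance, not within it.
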(fn PerformConditionCheckAI
  (params (OwnerController :type AI%20Controller%20Object%20Reference) (ControlledPawn :type Pawn%20Object%20Reference))
  (bind _asmonster_aicontroller_bp (Utilities|Casting|CastToMonsterAIController_BP OwnerController))
  (Variables|Default|SetMonster_AI_CON_REF _asmonster_aicontroller_bp)
  (return (>= (Math|Vector|VectorLength (- (Transformation|GetActorLocation (AI|BehaviorTree|GetBlackboardValueasActor (Variables|Default|GetTargetToFollow))) (Transformation|GetActorLocation (Pawn|GetControlledPawn (Variables|Default|GetMonster_AI_CON_REF))))) (Variables|Default|GetAcceptedDistance))))