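; Behavior Tree task that makes the monster chase the actor stored in the TargetToFollow blackboard key, intended to be the player.
; On execute it casts the owning controller to MyMonsterAIController on first use and caches it.
; It then runs AIMoveTo on the controlled pawn toward that actor with a small acceptance radius.
; The task finishes successfully on arrival; move failure has no handler, so it never calls FinishExecute in that case.
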(event EventReceiveExecuteAI
  (params (OwnerController :type AI%20Controller%20Object%20Reference) (ControlledPawn :type Pawn%20Object%20Reference))
  (if (!= (Variables|Default|GetMonster_AI_CON_Ref) 0)
    _
    (else
      (bind _asmy_monster_aicontroller (Utilities|Casting|CastToMyMonsterAIController OwnerController))
      (Variables|Default|SetMonster_AI_CON_Ref _asmy_monster_aicontroller)))
  (AI|AIMoveTo (Pawn|GetControlledPawn (Variables|Default|GetMonster_AI_CON_Ref)) "0, 0, 0" (AI|BehaviorTree|GetBlackboardValueasActor (Variables|Default|GetTargetToFollow)) 5e+01 false ; Moves Monster to character position
    (:OnSuccess
      (AI|BehaviorTree|FinishExecute true) ; When reached character position,  finish task and return to root
    )))