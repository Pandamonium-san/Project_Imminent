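; Behavior tree task in which the monster AI kills the player character.
; On execute it immediately calls Death on all player characters, prints the path length to the TargetToFollow blackboard actor, and flags the monster's kill as initialised.
; It switches the monster to flying movement and moves it to the target.
; Move success or failure both restore walking, reset the kill variables for debugging, and finish the task successfully.
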(event EventReceiveExecuteAI
  (params (OwnerController :type AI%20Controller%20Object%20Reference) (ControlledPawn :type Pawn%20Object%20Reference))
  (bind _targettofollow (Variables|Default|GetTargetToFollow))
  (bind _returnvalue (AI|BehaviorTree|GetBlackboardValueasActor _targettofollow))
  (bind _outactors (Actor|GetAllActorsOfClass "/Game/ImminentCPP/Blueprints/Project_ImminentCharacter_BP.Project_ImminentCharacter_BP_C"))
  (Default|Death _outactors)
  (bind _asmonster_aicontroller_bp (Utilities|Casting|CastToMonsterAIController_BP OwnerController))
  (Development|PrintString (Utilities|String|ToString(Float) (.PathLength (Class|NavigationSystem|GetPathLength (Transformation|GetActorLocation (Pawn|GetControlledPawn _asmonster_aicontroller_bp)) (Transformation|GetActorLocation _returnvalue)))) true true "(R=0.000000,G=0.660000,B=1.000000,A=1.000000)" 0.0)
  (bind _asmonster_bp (Utilities|Casting|CastToMonster_BP ControlledPawn))
  (Variables|/Game/ImminentCPP/Blueprints/AI/Monster_BP.Monster_BP_C|SetKillInitialised _asmonster_bp true)
  (Pawn|Components|CharacterMovement|SetMovementMode (Variables|/Script/Engine.Character|GetCharacterMovement _asmonster_bp) "MOVE_Flying" 0)
  (AI|AIMoveTo (Pawn|GetControlledPawn _asmonster_aicontroller_bp) "0.000000,0.000000,0.000000" _returnvalue 5e+01 true ; Moves Monster to character position
    (:OnSuccess
      _)
    (:OnFail
      _))
  (Development|PrintString "Die die die")
  ;[1 1 1] Reset for when debugging
  (Pawn|Components|CharacterMovement|SetMovementMode (Variables|/Script/Engine.Character|GetCharacterMovement _asmonster_bp) "MOVE_Walking" 0)
  (Variables|/Game/ImminentCPP/Blueprints/AI/Monster_BP.Monster_BP_C|SetKillInitialised _asmonster_bp false)
  (Variables|/Game/ImminentCPP/Blueprints/AI/Monster_BP.Monster_BP_C|SetKillFloat _asmonster_bp 0.0)
  (AI|BehaviorTree|FinishExecute true))