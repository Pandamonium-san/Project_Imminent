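; Monster character Blueprint that handles movement-driven footsteps, a kill-state speed boost and snuffing out nearby lights.
; Tick raises fly speed while KillInitialised is set, ramps KillFloat as a smooth jump-kill transition, and accumulates distance moved to trigger footsteps.
; PlayFootstep traces downward and picks a water or wood sound by surface type for the Audio component.
; The BP_LightKill overlap volume kills PointLight_killable actors on entry and rekindles them on exit.
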(event OnComponentBeginOverlap(BP_LightKill)
  (params (OverlappedComponent :type Primitive%20Component%20Object%20Reference) (OtherActor :type Actor%20Object%20Reference) (OtherComp :type Primitive%20Component%20Object%20Reference) (OtherBodyIndex :type Integer) (bFromSweep :type Boolean) (SweepResult :type Hit%20Result%20Structure%20%28by%20ref%29))
  (bind _aspoint_light_killable (Utilities|Casting|CastToPointLight_killable OtherActor))
  (Default|KillLight _aspoint_light_killable))

(event OnComponentEndOverlap(BP_LightKill)
  (params (OverlappedComponent :type Primitive%20Component%20Object%20Reference) (OtherActor :type Actor%20Object%20Reference) (OtherComp :type Primitive%20Component%20Object%20Reference) (OtherBodyIndex :type Integer))
  (bind _aspoint_light_killable (Utilities|Casting|CastToPointLight_killable OtherActor))
  (Default|Rekindle _aspoint_light_killable))

(event EventBeginPlay
  (Variables|Default|SetMaxWalkSpeed (Variables|/Script/Engine.CharacterMovementComponent|GetMaxWalkSpeed (Variables|Character|GetCharacterMovement))))

(event Collision|EventActorBeginOverlap
  (params (OtherActor :type Actor%20Object%20Reference)))

(event EventTick
  (params (DeltaSeconds :type Float%20%28single-precision%29))
  (bind _returnvalue (Transformation|GetVelocity))
  (bind _charactermovement (Variables|Character|GetCharacterMovement))
  (if (Variables|Default|GetKillInitialised)
    (Variables|/Script/Engine.CharacterMovementComponent|SetMaxFlySpeed _charactermovement 7e+02)
    ;[1 1 1] Smooth transition float for jumpKill
    (Variables|Default|SetKillFloat (Math|Interpolation|FInterptoConstant (Variables|Default|GetKillFloat) 1.0 (Utilities|Time|GetWorldDeltaSeconds) 2.0))
    (else
      (Variables|/Script/Engine.CharacterMovementComponent|SetMaxFlySpeed _charactermovement 4e+02)))
  ;[1 1 1] Footstep sounds
  (if (Math|Vector|NotEqual(Vector) _returnvalue "0, 0, 0" 0.0001)
    (bind _output_get (Variables|Default|SetStepCounter (+ (stale _output_get) (Math|Float|Clamp(Float) (* (Math|Vector|VectorLength _returnvalue) DeltaSeconds) 0.0 5.0))))
    (if (>= _output_get (Variables|Default|GetStepLength))
      (CallFunction|PlayFootstep)
      (Variables|Default|SetStepCounter 0.0))))

(fn ConstructionScript)

(fn PlayFootstep
  (bind _returnvalue (Transformation|GetActorLocation))
  (bind _audio (Variables|Default|GetAudio))
  (bind (_outhit _returnvalue_2) (Collision|LineTraceByChannel _returnvalue (+ _returnvalue "0, 0,-120.000000") "TraceTypeQuery1" false 0 "None"))
  (if _returnvalue_2
    (Audio|Components|Audio|SetSound _audio (Utilities|Select :Index (Collision|GetSurfaceType _outhit) :SurfaceType_Default "/Game/ImminentContent/Audio/Footsteps/Footstep_wood_monster.Footstep_wood_monster" :SurfaceType1 "/Game/ImminentContent/Audio/Footsteps/Footstep_wood_monster.Footstep_wood_monster" :SurfaceType2 "/Game/ImminentContent/Audio/Footsteps/Footstep_wood_monster.Footstep_wood_monster" :SurfaceType3 "/Game/ImminentContent/Audio/Footsteps/Footstep_wood_monster.Footstep_wood_monster" :SurfaceType4 "/Game/ImminentContent/Audio/Footsteps/Footstep_water_monster.Footstep_water_monster"))
    (Audio|Components|Audio|Play _audio 0.0)))