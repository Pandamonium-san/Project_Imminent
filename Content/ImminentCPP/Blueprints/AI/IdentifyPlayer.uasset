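; IdentifyPlayer is a Behavior Tree node that feeds the monster AI the player target it needs for chasing.
; On each AI tick it casts the owner to MonsterAIController_BP, caching that controller and the monster's location.
; It then loops over every Project_ImminentCharacter_BP actor, writing each to TargetToFollow and its position to TargetLocation.
; There is no distance or sight check, so the last actor found becomes the target.
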(event EventReceiveTickAI
  (params (OwnerController :type AI%20Controller%20Object%20Reference) (ControlledPawn :type Pawn%20Object%20Reference) (DeltaSeconds :type Float%20%28single-precision%29))
  ;[1 1 1] Setting up the AI controller to monster as a saved variable
  (bind _asmonster_aicontroller_bp (Utilities|Casting|CastToMonsterAIController_BP OwnerController))
  (Variables|Default|SetMonster_AI_Con_ref _asmonster_aicontroller_bp)
  (Variables|Default|SetMyLocation (Transformation|GetActorLocation (Pawn|GetControlledPawn (Variables|Default|GetMonster_AI_Con_ref))))
  ;[1 1 1] Sending the values to the blackboard which the monster needs to chase the player
  (bind _outactors (Actor|GetAllActorsOfClass "/Game/ImminentCPP/Blueprints/Project_ImminentCharacter_BP.Project_ImminentCharacter_BP_C"))
  (for _array_element _outactors
    (Class|BTFunctionLibrary|SetBlackboardValueasObject (Variables|Default|GetTargetToFollow) _array_element)
    (AI|BehaviorTree|SetBlackboardValueasVector (Variables|Default|GetTargetLocation) (Transformation|GetActorLocation _array_element))))