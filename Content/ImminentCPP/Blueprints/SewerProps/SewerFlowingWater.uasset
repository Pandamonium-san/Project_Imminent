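; Sewer water actor that switches between slow and fast flow, pushing things caught in it while fast.
; ChangeFlowSpeed swaps the water material and triggers a timeline, played or reversed, that shifts the water's height.
; A box overlap tracks root components of the player character and physics objects.
; While fast, Tick pushes them along the actor's forward vector: mass-divided impulses for physics bodies, LaunchCharacter plus Swimming mode for the character.
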(event OnComponentBeginOverlap(Box)
  (params (OverlappedComponent :type Primitive%20Component%20Object%20Reference) (OtherActor :type Actor%20Object%20Reference) (OtherComp :type Primitive%20Component%20Object%20Reference) (OtherBodyIndex :type Integer) (bFromSweep :type Boolean) (SweepResult :type Hit%20Result%20Structure%20%28by%20ref%29))
  (bind _returnvalue (VehicleSound|GetRootComponent OtherActor))
  (if (and (not (Utilities|Array|ContainsItem (Variables|Default|GetAffectedActors) _returnvalue)) (or (== (Utilities|GetClass OtherActor) "/Game/ImminentCPP/Blueprints/Project_ImminentCharacter_BP.Project_ImminentCharacter_BP_C") (Physics|IsSimulatingPhysics OtherComp "None")))
    (Utilities|Array|Add (Variables|Default|GetAffectedActors) _returnvalue)))

(event OnComponentEndOverlap(Box)
  (params (OverlappedComponent :type Primitive%20Component%20Object%20Reference) (OtherActor :type Actor%20Object%20Reference) (OtherComp :type Primitive%20Component%20Object%20Reference) (OtherBodyIndex :type Integer))
  (Utilities|Array|RemoveItem (Variables|Default|GetAffectedActors) (VehicleSound|GetRootComponent OtherActor))
  (Development|PrintText "out water"))

(event EventBeginPlay
  (Variables|Default|SetInitial%20position (Transformation|GetActorLocation))
  (Actor|Tick|SetActorTickEnabled true))

(event Collision|EventActorBeginOverlap
  (params (OtherActor :type Actor%20Object%20Reference)))

(event EventTick
  (params (DeltaSeconds :type Float%20%28single-precision%29))
  (if (Variables|Default|GetIsFast)
    (CallFunction|MoveActors DeltaSeconds))
  (if (Variables|Default|GetFlowIsChanging)
    (if (Variables|Default|GetIsFast)
      (bind _waterheight (Timeline|ChangeTimeline Play)
        (:Update
          (Transformation|SetActorLocation (+ (Variables|Default|GetInitial%20position) (Math|Vector|MakeVector 0.0 0.0 _waterheight)) false false))
        (:Finished
          (Variables|Default|SetFlowIsChanging false)))
      (else
        (Timeline|ChangeTimeline Reverse)))))

(fn ConstructionScript)

(fn ChangeFlowSpeed
  (params (Fast :type Boolean))
  (bind _staticmesh (Variables|Default|GetStaticMesh))
  (if (not (Variables|Default|GetFlowIsChanging))
    (bind _output_get (Variables|Default|SetIsFast Fast))
    (if _output_get
      (Rendering|Material|SetMaterial _staticmesh 0 "/Game/ImminentContent/Materials/Water/M_Water_Sewer_fast.M_Water_Sewer_fast")
      (else
        (Rendering|Material|SetMaterial _staticmesh 0 "/Game/ImminentContent/Materials/Water/M_Water_Sewer_slow.M_Water_Sewer_slow")))
    (Variables|Default|SetFlowIsChanging true)))

(fn MoveActors
  (params (Delta :type Float%20%28single-precision%29))
  (for _array_element (Variables|Default|GetAffectedActors)
    (bind _asprimitive_component (Utilities|Casting|CastToPrimitiveComponent _array_element))
    (if (Physics|IsSimulatingPhysics _asprimitive_component "None")
      (Physics|AddImpulse _asprimitive_component (* (/ (* (* (Transformation|GetActorForwardVector) (Variables|Default|GetFlowForce)) Delta) (Physics|GetMass _asprimitive_component)) 4e+03) "None" false)
      (else
        (bind _asproject_imminent_character_bp (Utilities|Casting|CastToProject_ImminentCharacter_BP (Components|GetOwner _array_element)))
        (Character|LaunchCharacter _asproject_imminent_character_bp (* (* (Transformation|GetActorForwardVector) (/ (Variables|Default|GetFlowForce) 8e+01)) Delta) false false)
        (Pawn|Components|CharacterMovement|SetMovementMode (Variables|/Script/Engine.Character|GetCharacterMovement _asproject_imminent_character_bp) "MOVE_Swimming" 0)))))