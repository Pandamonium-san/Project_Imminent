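; Sewer prop Blueprint that builds a cable along an editable spline.
; The construction script walks the spline's length in small fixed distance steps, adding an SM_Cable_Piece_3 static mesh component at each point, rotated along the spline direction.
; An iteration counter forces the loop to end after a hard cap, and leftover time-based sampling logic is unused.
; The event graph has no active logic.
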(event EventBeginPlay)

(event Collision|EventActorBeginOverlap
  (params (OtherActor :type Actor%20Object%20Reference)))

(event EventTick
  (params (DeltaSeconds :type Float%20%28single-precision%29)))

(fn ConstructionScript
  (bind _itr (LocalVariables|GetItr))
  (bind _spline (Variables|Default|GetSpline))
  (LocalVariables|SetTotalLength (Spline|GetSplineLength _spline))
  (while (<= (LocalVariables|GetDistance) (LocalVariables|GetTotalLength))
    (bind _returnvalue (AddComponent|AddStaticMeshComponent false (Math|Transform|MakeTransform (Spline|GetLocationatDistanceAlongSpline _spline (LocalVariables|GetDistance) "Local") (Math|Conversions|RotationFromXVector (Spline|GetDirectionatDistanceAlongSpline _spline (LocalVariables|GetDistance) "Local")))))
    (Components|StaticMesh|SetStaticMesh _returnvalue "/Game/ImminentContent/Meshes/SM_Cable_Piece_3.SM_Cable_Piece_3")
    (Transformation|AttachComponentToComponent _returnvalue (Variables|Default|GetSpline) "None" "KeepRelative" "KeepRelative" "KeepRelative" true)
    (bind _output_get (LocalVariables|SetDistance (+ (stale _output_get) 2.0)))
    (Math|Integer|IncrementInt _itr
      (:%20%20
        (if (> _itr 10000)
          (LocalVariables|SetTime 999999.0)
          (LocalVariables|SetDistance 99999999.0))))))