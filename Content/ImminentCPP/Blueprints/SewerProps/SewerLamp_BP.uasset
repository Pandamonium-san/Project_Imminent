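; SewerLamp_BP is a sewer lamp prop that shows whether its light is on or off through its glass material.
; It overrides the LightOn and LightOff events, calling the parent version before swapping material slot 0 on the static mesh between the on and off glass materials.
; Each event also prints its state as debug text, while the remaining event stubs and construction script add no behavior of their own.
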(event EventBeginPlay
  (|CallParentFunction))

(event Collision|EventActorBeginOverlap
  (params (OtherActor :type Actor%20Object%20Reference)))

(event EventTick
  (params (DeltaSeconds :type Float%20%28single-precision%29)))

(event EventLighton
  (|CallParentFunction)
  (Rendering|Material|SetMaterial (Variables|Default|GetStaticMesh) 0 "/Game/ImminentContent/Materials/LampGlass/M_SewerLampGlass_on.M_SewerLampGlass_on")
  (Development|PrintText "on"))

(event EventLightOff
  (|CallParentFunction)
  (Rendering|Material|SetMaterial (Variables|Default|GetStaticMesh) 0 "/Game/ImminentContent/Materials/LampGlass/M_SewerLampGlass_off.M_SewerLampGlass_off")
  (Development|PrintText "off"))

(fn ConstructionScript
  (|CallParentFunction))