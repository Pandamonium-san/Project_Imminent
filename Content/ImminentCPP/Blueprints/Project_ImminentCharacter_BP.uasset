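; First-person player character Blueprint that adds the HUD, footsteps, running camera effects and the death and respawn sequence.
; Tick accumulates walked distance to trigger footsteps, using a downward trace to pick the sound by physical surface.
; While running, a timeline changes FOV and head-bob shake plays when walking.
; Death plays a level sequence with input and movement disabled, blacks out the camera, calls RespawnAtCheckpoint, then restores control after a delay.
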(event Custom|Death
  ;[1 1 1] Death
  (Variables|Default|SetCameraPos (Variables|/Script/Engine.SceneComponent|GetRelativeLocation (Variables|Default|GetFirstPersonCameraComponent)))
  (Utilities|FlowControl|Sequence
    (:then_0
      (Utilities|FlowControl|DoOnce false
        (:Completed
          (Input|DisableInput (Game|Player|GetPlayerPawn 0) 0)
          (bind _returnvalue (Sequencer|Player|CreateLevelSequencePlayer "/Game/ImminentCPP/Blueprints/DeathScene_1.DeathScene_1"))
          (Variables|/Script/Engine.CameraComponent|SetbUsePawnControlRotation (Variables|Default|GetFirstPersonCameraComponent) false)
          (Pawn|Components|CharacterMovement|SetMovementMode (Variables|Character|GetCharacterMovement) "MOVE_None" 0)
          (Audio|Components|Audio|Play _returnvalue))))
    (:then_1
      (Utilities|FlowControl|Delay (Class|LevelSequencePlayer|GetLength _returnvalue))
      (Variables|/Script/Engine.CameraComponent|SetPostProcessSettings (Variables|Default|GetFirstPersonCameraComponent) (Utilities|Struct|MakePostProcessSettings "(R=0.000000,G=0.000000,B=0.000000,A=1.000000)"))
      (Class|ProjectImminentCharacter|RespawnatCheckpoint)
      (Utilities|FlowControl|Delay 3.0)
      (Input|EnableInput (Game|Player|GetPlayerPawn 0) 0)
      (Variables|/Script/Engine.CameraComponent|SetbUsePawnControlRotation (Variables|Default|GetFirstPersonCameraComponent) true)
      (Pawn|Components|CharacterMovement|SetMovementMode (Variables|Character|GetCharacterMovement) "MOVE_Walking" 0)
      (Transformation|SetRelativeLocation (Variables|Default|GetFirstPersonCameraComponent) (Variables|Default|GetCameraPos) false false)
      (Variables|/Script/Engine.CameraComponent|SetPostProcessSettings (Variables|Default|GetFirstPersonCameraComponent) (Utilities|Struct|MakePostProcessSettings "(R=1.000000,G=1.000000,B=1.000000,A=1.000000)")))))

(event EventBeginPlay
  (bind _returnvalue (UserInterface|CreateWidget "/Game/ImminentCPP/Blueprints/GUI/HUD.HUD_C"))
  (bind _output_get (Variables|Default|SetHUD%20Reference _returnvalue))
  (UserInterface|Viewport|AddtoViewport _output_get 0))

(event Collision|EventActorBeginOverlap
  (params (OtherActor :type Actor%20Object%20Reference)))

(event EventTick
  (params (DeltaSeconds :type Float%20%28single-precision%29))
  (bind _charactermovement (Variables|Character|GetCharacterMovement))
  (bind _movementmode (Variables|/Script/Engine.CharacterMovementComponent|GetMovementMode _charactermovement))
  (bind _returnvalue (Utilities|Select :Index _movementmode :MOVE_None false :MOVE_Walking true :MOVE_NavWalking false :MOVE_Falling false :MOVE_Swimming false :MOVE_Flying false :MOVE_Custom false))
  ;[1 1 1] Footstep sound
  (if _returnvalue
    (bind _output_get (Variables|Default|SetDistanceTravelled (+ (* DeltaSeconds (Math|Vector|VectorLength (Transformation|GetVelocity))) (stale _output_get))))
    (if (>= _output_get (Variables|Default|GetStepSize))
      (CallFunction|PlayFootstep)
      (else
        (if (Variables|Default|GetbRunning) :!label _label
          (if _returnvalue
            (Class|PlayerController|ClientPlayCameraShake (Game|GetPlayerController 0) "/Game/ImminentCPP/Blueprints/CameraShake_HeadBob.CameraShake_HeadBob_C" 1.0 "CameraLocal" "0, 0, 0")
            (bind _fov_track (Timeline|FoV_TimeLine Play)
              (:Update
                (Camera|SetFieldOfView (Variables|Default|GetFirstPersonCameraComponent) _fov_track)))
            (else
              (Timeline|FoV_TimeLine Play)))
          (else
            (Timeline|FoV_TimeLine Reverse)))))
    (else
      (Variables|Default|SetDistanceTravelled (Variables|Default|GetStepSize))
      (goto _label))))

(fn ConstructionScript)

(fn PlayFootstep
  (bind _returnvalue (Transformation|GetActorLocation))
  (bind (_outhit _returnvalue_2) (Collision|LineTraceByChannel (+ _returnvalue "0, 0,50.000000") (+ _returnvalue "0, 0,-170.000000") "TraceTypeQuery1" false 0 "None"))
  (if _returnvalue_2
    (Audio|PlaySoundatLocation (Utilities|Select :Index (Collision|GetSurfaceType _outhit) :SurfaceType_Default "/Game/ImminentContent/Audio/Footsteps/Footstep_concrete.Footstep_concrete" :SurfaceType1 "/Game/ImminentContent/Audio/Footsteps/Footstep_concrete.Footstep_concrete" :SurfaceType2 "/Game/ImminentContent/Audio/Footsteps/Footstep_wood.Footstep_wood" :SurfaceType3 "/Game/ImminentContent/Audio/Footsteps/Footstep_gravel.Footstep_gravel" :SurfaceType4 "/Game/ImminentContent/Audio/Footsteps/Footstep_water.Footstep_water") (.Location (Collision|BreakHitResult _outhit)))
    (Variables|Default|SetDistanceTravelled 0.0)))