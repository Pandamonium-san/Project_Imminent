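; Cart Blueprint that moves its static mesh along a rail spline in increments, one push each time it is triggered.
; TriggerEvent disables the CartTrigger, stores the current spline time as the new start and resets the RailSpline timeline.
; Tick keeps playing that timeline, which offsets spline time by PushDistance, updates the mesh's location and rotation, and re-enables the trigger when finished.
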(event Custom|TriggerEvent
  (bind _spline (Variables|Default|GetSpline))
  (Variables|/Script/Project_Imminent.TriggerComponent|SetUserInteractable (Variables|Default|GetCartTrigger) false)
  (Variables|Default|SetPrevSplineTime (Variables|Default|GetCurrentSplineTime))
  (bind _splinetime (Timeline|RailSpline SetNewTime)
    (:Update
      (bind _output_get (Variables|Default|SetCurrentSplineTime (+ (Variables|Default|GetPrevSplineTime) (* _splinetime (Variables|Default|GetPushDistance)))))
      (Transformation|SetWorldLocationAndRotation (Variables|Default|GetStaticMesh) (Spline|GetLocationatTime _spline _output_get "World" false) (Class|SplineComponent|GetRotationatTime _spline _output_get "Local" false) false false))
    (:Finished
      (Variables|/Script/Project_Imminent.TriggerComponent|SetUserInteractable (Variables|Default|GetCartTrigger) true))))

(event EventBeginPlay)

(event Collision|EventActorBeginOverlap
  (params (OtherActor :type Actor%20Object%20Reference)))

(event EventTick
  (params (DeltaSeconds :type Float%20%28single-precision%29))
  (bind _spline (Variables|Default|GetSpline))
  (bind _splinetime (Timeline|RailSpline Play)
    (:Update
      (bind _output_get (Variables|Default|SetCurrentSplineTime (+ (Variables|Default|GetPrevSplineTime) (* _splinetime (Variables|Default|GetPushDistance)))))
      (Transformation|SetWorldLocationAndRotation (Variables|Default|GetStaticMesh) (Spline|GetLocationatTime _spline _output_get "World" false) (Class|SplineComponent|GetRotationatTime _spline _output_get "Local" false) false false))
    (:Finished
      (Variables|/Script/Project_Imminent.TriggerComponent|SetUserInteractable (Variables|Default|GetCartTrigger) true))))

(fn ConstructionScript)