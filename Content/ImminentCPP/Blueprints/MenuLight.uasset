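; MenuLight is a flickering lantern actor, apparently for the menu scene, pairing a point light with a static mesh.
; The construction script gives the glass slot a dynamic M_LanternGlass instance with a faint emissive glow.
; Each tick has a small random chance to cut both light and glow, then a timer relights them after a random delay of up to a second.
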(event Custom|Relight
  (Rendering|Components|Light|SetIntensity (Variables|Default|GetPointLight) (Variables|Default|GetInitial%20Intensity))
  (Rendering|Material|SetScalarParameterValue (Variables|Default|GetLanternDMI) "Emissive Power" 0.1 :!class /Script/Engine.MaterialInstanceDynamic))

(event EventBeginPlay
  (Variables|Default|SetInitial%20Intensity (Variables|/Script/Engine.LightComponentBase|GetIntensity (Variables|Default|GetPointLight))))

(event Collision|EventActorBeginOverlap
  (params (OtherActor :type Actor%20Object%20Reference)))

(event EventTick
  (params (DeltaSeconds :type Float%20%28single-precision%29))
  (if (< (Math|Random|RandomFloatinRange 0.0 1.0) 0.01)
    (Rendering|Components|Light|SetIntensity (Variables|Default|GetPointLight) 0.0)
    (Rendering|Material|SetScalarParameterValue (Variables|Default|GetLanternDMI) "Emissive Power" 0.0 :!class /Script/Engine.MaterialInstanceDynamic)
    (Utilities|Time|SetTimerbyEvent (delegate Custom|Relight) (Math|Random|RandomFloatinRange 0.0 1.0))))

(fn ConstructionScript
  (bind _returnvalue (Rendering|Material|CreateDynamicMaterialInstance "/Game/ImminentContent/Materials/LampGlass/M_LanternGlass.M_LanternGlass" :!class /Script/Engine.KismetMaterialLibrary))
  (bind _output_get (Variables|Default|SetLanternDMI _returnvalue))
  (Rendering|Material|SetMaterial (Variables|Default|GetStaticMesh) 5 _output_get)
  (Rendering|Material|SetScalarParameterValue _output_get "Emissive Power" 0.1 :!class /Script/Engine.MaterialInstanceDynamic))