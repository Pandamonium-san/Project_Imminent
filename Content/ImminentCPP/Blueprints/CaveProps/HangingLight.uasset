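; HangingLight is a hanging lamp prop for the caves whose glass glows and goes dark with its light.
; On BeginPlay it puts a dynamic M_LampGlass material instance on SphereLight with a faint emissive glow.
; When Flickers is set, the on and off events call the parent light logic and toggle that glow; otherwise both do nothing.
; The construction script assigns a bulb-smash cue as the light-out sound.
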(event EventBeginPlay
  (|CallParentFunction)
  (bind _returnvalue (Rendering|Material|CreateDynamicMaterialInstance "/Game/ImminentContent/Materials/LampGlass/M_LampGlass.M_LampGlass" :!class /Script/Engine.KismetMaterialLibrary))
  (bind _output_get (Variables|Default|SetDynamic%20Material%20Instance _returnvalue))
  (Rendering|Material|SetMaterial (Variables|Default|GetSphereLight) 0 _output_get)
  (Rendering|Material|SetScalarParameterValue _output_get "Emissive Power" 0.05 :!class /Script/Engine.MaterialInstanceDynamic))

(event Collision|EventActorBeginOverlap
  (params (OtherActor :type Actor%20Object%20Reference)))

(event EventTick
  (params (DeltaSeconds :type Float%20%28single-precision%29))
  (|CallParentFunction 0.0))

(event EventLighton
  (if (Variables|Default|GetFlickers)
    (|CallParentFunction)
    (Rendering|Material|SetScalarParameterValue (Variables|Default|GetDynamic%20Material%20Instance) "Emissive Power" 0.05 :!class /Script/Engine.MaterialInstanceDynamic)))

(event EventLightOff
  (params (PlaySound :type Boolean))
  (if (Variables|Default|GetFlickers)
    (|CallParentFunction PlaySound)
    (Rendering|Material|SetScalarParameterValue (Variables|Default|GetDynamic%20Material%20Instance) "Emissive Power" 0.0 :!class /Script/Engine.MaterialInstanceDynamic)))

(fn ConstructionScript
  (|CallParentFunction)
  (Variables|Default|SetLightOut%20Sound "/Game/ImminentContent/Audio/LightBulbSmash_Cue.LightBulbSmash_Cue"))