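; SwitchTrigger is a trigger component that acts as a switch, relaying its trigger event to other trigger components.
; It can fire from an optionally looping timer or from owner begin/end overlaps that pass a class comparison.
; Triggering calls components on target actors, plus owner components selected by class or index, then runs the parent event.
; A DoOnce option turns off user interaction after the first trigger.
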(event Custom|OverlapEvent
  (params (OverlappedActor :type Actor%20Object%20Reference) (OtherActor :type Actor%20Object%20Reference))
  (if (== (Utilities|GetClass OtherActor) (Variables|Default|GetOtherActor))
    (Class|TriggerComponent|TriggerEvent)))

(event EventBeginPlay
  (bind _returnvalue (Components|GetOwner))
  (if (Variables|Timer|GetTimed)
    (Utilities|Time|SetTimerbyEvent (delegate EventTriggerEvent) (Variables|Timer|GetTime) (Variables|Timer|GetLooping)))
  (if (Variables|Default|GetTriggerOnActorBeginOverlap)
    (Collision|BindEventtoOnActorBeginOverlap _returnvalue (delegate Custom|OverlapEvent)))
  (if (Variables|Default|GetTriggerOnActorEndOverlap)
    (Collision|BindEventtoOnActorEndOverlap _returnvalue (delegate Custom|OverlapEvent))))

(event EventTick
  (params (DeltaSeconds :type Float%20%28single-precision%29)))

(event EventTriggerEvent
  (if (Variables|Default|GetDoOnce)
    (Utilities|FlowControl|DoOnce false
      (:Completed
        (Variables|Default|SetUserInteractable false))))
  (for _array_element (Variables|Default|GetTargetActors)
    (for _array_element_2 (Actor|GetComponentsByClass _array_element "/Script/Project_Imminent.TriggerComponent")
      (Class|TriggerComponent|TriggerEvent _array_element_2)))
  (for _array_element_3 (Variables|Default|GetTargetComponents)
    (Class|TriggerComponent|TriggerEvent (Actor|GetComponentbyClass (Components|GetOwner) _array_element_3)))
  (bind _output_get (Variables|Default|SetTargets (Actor|GetComponentsByClass (Components|GetOwner) "/Script/Project_Imminent.TriggerComponent")))
  (for _array_element_4 (Variables|Default|GetTargetComponentIndex)
    (Class|TriggerComponent|TriggerEvent (Utilities|Array|Get(acopy) _output_get _array_element_4)))
  (|CallParentFunction))