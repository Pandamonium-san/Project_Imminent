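; Trigger component that fractures its owning DestructibleActor when TriggerEvent fires.
; A DoOnce lets it run a single time, enabling physics on the destructible component and playing a low-pitched, attenuated explosion cue there.
; It then applies damage at the component's location using its damage and impulse variables before calling the parent TriggerEvent.
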(event EventBeginPlay)

(event EventTick
  (params (DeltaSeconds :type Float%20%28single-precision%29)))

(event EventTriggerEvent
  (Utilities|FlowControl|DoOnce false
    (:Completed
      (bind _asdestructible_actor (Utilities|Casting|CastToDestructibleActor (Components|GetOwner)))
      (Physics|SetSimulatePhysics (Variables|/Script/Engine.DestructibleActor|GetDestructibleComponent _asdestructible_actor) true)
      (Audio|PlaySoundatLocation "/Game/StarterContent/Audio/Explosion_Cue.Explosion_Cue" (Transformation|GetWorldLocation (Variables|/Script/Engine.DestructibleActor|GetDestructibleComponent _asdestructible_actor)) "0, 0, 0" 0.5 0.4 0.0 "/Game/ImminentContent/Audio/Attenuation/Monster_Attenuation.heartbeat_attenuation")
      (Game|Damage|ApplyDamage (Variables|/Script/Engine.DestructibleActor|GetDestructibleComponent _asdestructible_actor) (Variables|Default|GetDamage%20Amount) (Transformation|GetWorldLocation (Variables|/Script/Engine.DestructibleActor|GetDestructibleComponent _asdestructible_actor)) (Variables|Default|GetImpulse%20Dir) (Variables|Default|GetImpulse%20Strength))
      (|CallParentFunction))))