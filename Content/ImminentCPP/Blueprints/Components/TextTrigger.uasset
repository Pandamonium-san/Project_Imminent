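; TextTrigger shows a sequence of help text lines and a key set on the player's HUD when TriggerEvent fires.
; TriggerEvent uses the HUD reference, fetching it from the player's Project_ImminentCharacter_BP if not yet valid, then restarts the sequence.
; ShowNext draws the current line with optional fades, then re-schedules itself by timer after the display and enabled fade times until the text array ends.
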(event Custom|ShowNext
  (bind _hud_reference (Variables|Default|GetHUD_Reference))
  (Default|DrawKeys _hud_reference (Variables|Default|GetKeySet))
  (Default|DrawHelpText _hud_reference (Utilities|Array|Get(acopy) (Variables|Default|GetText) (Variables|Default|GetIterator)) (+ (Variables|Default|GetTime) 0.001) (Variables|Default|GetFadeTime) (Variables|Default|GetFadeIn) (Variables|Default|GetFadeOut))
  (Math|Integer|IncrementInt (Variables|Default|GetIterator)
    (:%20%20
      (if (< (Variables|Default|GetIterator) (Utilities|Array|Length (Variables|Default|GetText)))
        (Utilities|Time|SetTimerbyEvent (delegate Custom|ShowNext) (+ (* (Variables|Default|GetFadeTime) (+ (Math|Conversions|ToFloat(Boolean) (Variables|Default|GetFadeOut)) (Math|Conversions|ToFloat(Boolean) (Variables|Default|GetFadeIn)))) (Variables|Default|GetTime)))))))

(event EventBeginPlay)

(event EventTick
  (params (DeltaSeconds :type Float%20%28single-precision%29)))

(event EventTriggerEvent
  (Utilities|IsValid (Variables|Default|GetHUD_Reference)
    (:Is%20Valid
      (Variables|Default|SetIterator 0 :!label _label)
      (CallFunction|ShowNext))
    (:Is%20Not%20Valid
      (bind _asproject_imminent_character_bp (Utilities|Casting|CastToProject_ImminentCharacter_BP (Game|GetPlayerCharacter 0))
        (:then
          (Variables|Default|SetHUD_Reference (Variables|/Game/ImminentCPP/Blueprints/Project_ImminentCharacter_BP.Project_ImminentCharacter_BP_C|GetHUD%20Reference _asproject_imminent_character_bp))
          (goto _label))
        (:CastFailed
          (Development|PrintText "TextTrigger cast to Project_ImminentCharacter_BP failed."))))))