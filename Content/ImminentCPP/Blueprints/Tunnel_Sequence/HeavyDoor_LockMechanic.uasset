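; HeavyDoor_LockMechanic is the gear lock for the heavy cave door in the tunnel sequence.
; When its HeavyCaveDoorTrigger component activates, it plays a metal click, then after a short delay a door sound at the first HeavyCaveDoor_BP found, plus a mini-earthquake camera shake.
; It then hides the loose wheel, shows Wheel1, and plays a timeline that spins the three wheels, with the middle one turning opposite to the others.
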(event OnComponentActivated(HeavyCaveDoorTrigger)
  (params (bReset :type Boolean))
  (Audio|PlaySoundatLocation "/Game/ImminentContent/Audio/_littleluigi_1-metal-click_converted._littleluigi_1-metal-click_converted" (Transformation|GetActorLocation) "0, 0, 0" 2.0 -1.0 1.0)
  (Utilities|FlowControl|Delay 0.1)
  (bind _outactors (Actor|GetAllActorsOfClass "/Game/ImminentCPP/Blueprints/Tunnel_Sequence/HeavyCaveDoor_BP.HeavyCaveDoor_BP_C"))
  (Audio|PlaySoundatLocation "/Game/ImminentContent/Audio/cavedoor_converted.cavedoor_converted" (Transformation|GetActorLocation (Utilities|Array|Get(acopy) _outactors)) "0, 0, 0" 0.8 1.0 0.0 "/Game/ImminentContent/Audio/Attenuation/Monster_Attenuation.Monster_attenuation")
  (Class|PlayerController|ClientPlayCameraShake (Game|GetPlayerController 0) "/Game/ImminentCPP/Blueprints/CameraShake_Mini_Earthquake.CameraShake_Mini_Earthquake_C" 0.3 "CameraLocal" "0, 0, 0")
  (Rendering|SetVisibility (Variables|Default|GetLooseWheel) false false)
  (Rendering|SetVisibility (Variables|Default|GetWheel1) true false)
  (Timeline|Timeline_0 Play
    (:Update
      (Transformation|AddLocalRotation (Variables|Default|GetWheel1) "0.000000,1.000000,0.000000" false false)
      (Transformation|AddLocalRotation (Variables|Default|GetWheel2) "0.000000,-1.000000,0.000000" false false)
      (Transformation|AddLocalRotation (Variables|Default|GetWheel3) "0.000000,1.000000,0.000000" false false))))

(event EventBeginPlay)

(event Collision|EventActorBeginOverlap
  (params (OtherActor :type Actor%20Object%20Reference)))

(event EventTick
  (params (DeltaSeconds :type Float%20%28single-precision%29)))

(fn ConstructionScript)