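; Sewer trigger Blueprint that shuts off the electrical spark hazards when its trigger event fires.
; It finds every actor of two spark Blueprint classes in the level, disables each one, and stops the sound on the first class.
; It then plays a metal click at the owner's location and calls the parent trigger event through a DoOnce, so only that parent call is limited to one run.
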(event EventBeginPlay)

(event EventTick
  (params (DeltaSeconds :type Float%20%28single-precision%29)))

(event EventTriggerEvent
  (bind _outactors (Actor|GetAllActorsOfClass "/Game/ImminentCPP/Blueprints/SewerProps/P_Sparks_3_Blueprint.P_Sparks_3_Blueprint_C"))
  (for _array_element _outactors
    (CallFunction|DisableActor _array_element)
    (Default|StopSound _array_element))
  (bind _outactors_2 (Actor|GetAllActorsOfClass "/Game/StarterContent/Blueprints/Blueprint_Effect_Sparks.Blueprint_Effect_Sparks_C"))
  (for _array_element_2 _outactors_2
    (CallFunction|DisableActor _array_element_2))
  (Audio|PlaySoundatLocation "/Game/ImminentContent/Audio/MetalClick_cue.MetalClick_cue" (Transformation|GetActorLocation (Components|GetOwner)))
  (Utilities|FlowControl|DoOnce false
    (:Completed
      (|CallParentFunction))))