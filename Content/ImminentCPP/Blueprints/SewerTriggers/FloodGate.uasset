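; FloodGate is a triggerable component that slides its owning actor vertically to act as a sewer flood gate.
; TriggerEvent is ignored during motion; otherwise it toggles Closed, plays the matching metal shake sound and calls the parent event.
; Tick drives Move with signed delta time, raising the actor when Closed and lowering it otherwise.
; Move interpolates linearly over RiseTime, then stores the new location as the next starting point.
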(event EventBeginPlay
  (bind _returnvalue (Components|GetOwner))
  (Variables|Default|SetActor _returnvalue)
  (Variables|Default|SetInitialLocation (Transformation|GetActorLocation _returnvalue)))

(event EventTick
  (params (DeltaSeconds :type Float%20%28single-precision%29))
  (if (Variables|Default|GetInMotion)
    (CallFunction|Move (* (Math|Integer|SelectInt 1 -1 (Variables|Default|GetClosed)) DeltaSeconds))))

(event EventTriggerEvent
  (if (not (Variables|Default|GetInMotion))
    (bind _output_get (Variables|Default|SetClosed (not (stale _output_get))))
    (Variables|Default|SetInMotion true)
    (Audio|PlaySoundatLocation (select _output_get "/Game/ImminentContent/Audio/MetalShaking/MetalShake_Close_Cue.MetalShake_Close_Cue" "/Game/ImminentContent/Audio/MetalShaking/MetalShake_Open_Cue.MetalShake_Open_Cue") (Transformation|GetActorLocation (Components|GetOwner)))
    (|CallParentFunction)))

(fn Move
  (params (Time :type Float%20%28single-precision%29))
  (bind _output_get (Variables|Default|SetCurrentTime (+ (stale _output_get) Time)))
  (Variables|Default|SetCurrentHeight (* (Variables|Default|GetRiseAmount) (/ (Variables|Default|GetCurrentTime) (Variables|Default|GetRiseTime))))
  (Transformation|SetActorLocation (Variables|Default|GetActor) (+ (Variables|Default|GetInitialLocation) (Math|Vector|MakeVector 0.0 0.0 (Variables|Default|GetCurrentHeight))) false false)
  (if (or (>= (Variables|Default|GetCurrentTime) (Variables|Default|GetRiseTime)) (<= (Variables|Default|GetCurrentTime) (* -1 (Variables|Default|GetRiseTime))))
    (Variables|Default|SetInMotion false)
    (Variables|Default|SetCurrentTime 0.0)
    (Variables|Default|SetInitialLocation (Transformation|GetActorLocation (Components|GetOwner)))))