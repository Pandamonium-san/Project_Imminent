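; EndGameTrigger is a collision trigger in the sewer triggers set that starts the end-game sequence when the player character overlaps it.
; The overlap disables player input and plays a referenced level sequence.
; After a short delay it hides the player, then moves existing Monster_BP actors to a preset relative position and rotation, commented as behind the player, rather than spawning new ones.
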(event OnComponentBeginOverlap(CollisionComponent)
  (params (OverlappedComponent :type Primitive%20Component%20Object%20Reference) (OtherActor :type Actor%20Object%20Reference) (OtherComp :type Primitive%20Component%20Object%20Reference) (OtherBodyIndex :type Integer) (bFromSweep :type Boolean) (SweepResult :type Hit%20Result%20Structure%20%28by%20ref%29))
  (bind _asproject_imminent_character_bp (Utilities|Casting|CastToProject_ImminentCharacter_BP OtherActor))
  (Input|DisableInput _asproject_imminent_character_bp 0)
  (Audio|Components|Audio|Play (Variables|/Script/LevelSequence.LevelSequenceActor|GetSequencePlayer (Variables|Default|GetSequence)))
  (Utilities|FlowControl|Delay 1.0)
  (Rendering|SetActorHiddenInGame _asproject_imminent_character_bp true)
  ;[1 1 1] Spawn Monster Behind Player
  (bind _outactors (Actor|GetAllActorsOfClass "/Game/ImminentCPP/Blueprints/AI/Monster_BP.Monster_BP_C"))
  (Transformation|SetActorRelativeLocation _outactors (Variables|Default|GetMonsterSpawnPos))
  (Transformation|SetActorRelativeRotation _outactors (Variables|Default|GetMonsterRotation)))

(event EventBeginPlay)

(event Collision|EventActorBeginOverlap
  (params (OtherActor :type Actor%20Object%20Reference)))

(event EventTick
  (params (DeltaSeconds :type Float%20%28single-precision%29)))

(fn ConstructionScript)