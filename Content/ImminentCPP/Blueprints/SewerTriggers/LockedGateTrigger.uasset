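; LockedGateTrigger handles interaction with a LockedGate that can only be opened from one side.
; When triggered, it takes the dot product of the owner-to-player offset and the gate's forward vector to find which side the player is on.
; From the front, the player's HUD shows a fading "locked from the other side" message.
; From the back, it opens the gate, disables further interaction and plays a metal click at the gate.
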(event EventBeginPlay)

(event EventTick
  (params (DeltaSeconds :type Float%20%28single-precision%29)))

(event EventTriggerEvent
  (bind _returnvalue (Components|GetOwner))
  (if (> (Math|Vector|DotProduct (- (Transformation|GetActorLocation (Game|GetPlayerCharacter 0)) (Transformation|GetActorLocation _returnvalue)) (Transformation|GetActorForwardVector _returnvalue)) 0.0)
    ;[1 1 1] Front
    (bind _asproject_imminent_character_bp (Utilities|Casting|CastToProject_ImminentCharacter_BP (Game|GetPlayerCharacter 0)))
    (Default|DrawHelpText (Variables|/Game/ImminentCPP/Blueprints/Project_ImminentCharacter_BP.Project_ImminentCharacter_BP_C|GetHUD%20Reference _asproject_imminent_character_bp) "It's locked from the other side" 2.0 1.0 true true)
    (else
      ;[1 1 1] Back
      (bind _aslocked_gate (Utilities|Casting|CastToLockedGate (Components|GetOwner)))
      (Default|Open _aslocked_gate)
      (Variables|Default|SetUserInteractable false)
      (Audio|SpawnSoundatLocation "/Game/ImminentContent/Audio/_littleluigi_1-metal-click_converted._littleluigi_1-metal-click_converted" (Transformation|GetActorLocation (Components|GetOwner))))))