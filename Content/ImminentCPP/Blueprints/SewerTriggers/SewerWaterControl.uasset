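; SewerWaterControl is a trigger that switches the flow speed of the sewer water between fast and normal.
; Its TriggerEvent gathers all SewerFlowingWater actors, calls ChangeFlowSpeed on each with the inverted IsFast state, then flips that flag.
; A DoOnce that resets after a short delay acts as a cooldown between toggles.
; The parent TriggerEvent call is left unconnected, so inherited trigger logic does not run.
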(event EventBeginPlay)

(event EventTick
  (params (DeltaSeconds :type Float%20%28single-precision%29)))

(event EventTriggerEvent
  (Utilities|FlowControl|DoOnce false :!label _label
    (:Completed
      (bind _outactors (Actor|GetAllActorsOfClass "/Game/ImminentCPP/Blueprints/SewerProps/SewerFlowingWater.SewerFlowingWater_C"))
      (bind _output_get (Variables|Default|SetSewerWater _outactors))
      (for _array_element _output_get
        (Default|ChangeFlowSpeed _array_element (not (Variables|Default|GetIsFast))))
      (Variables|Default|SetIsFast (not (Variables|Default|GetIsFast)))
      (Utilities|FlowControl|Delay 5.0)
      (goto _label Reset))))