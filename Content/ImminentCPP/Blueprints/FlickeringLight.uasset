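; FlickeringLight is a light actor that flickers at random, built on inherited or external LightOn and LightOff functions.
; Each tick it rolls a random number against Frequency and, on a hit, switches the light off and sets a one-shot timer of up to a second to relight it.
; The chance is per frame, so flicker rate depends on framerate, and a new hit during an outage resets the pending relight timer.
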(event Custom|Relight
  (CallFunction|Lighton))

(event EventBeginPlay
  (|CallParentFunction))

(event Collision|EventActorBeginOverlap
  (params (OtherActor :type Actor%20Object%20Reference)))

(event EventTick
  (params (DeltaSeconds :type Float%20%28single-precision%29))
  (if (< (Math|Random|RandomFloatinRange 0.0 1.0) (Variables|Default|GetFrequency))
    (CallFunction|LightOff false)
    (Utilities|Time|SetTimerbyEvent (delegate Custom|Relight) (Math|Random|RandomFloatinRange 0.0 1.0))))

(fn ConstructionScript
  (|CallParentFunction))