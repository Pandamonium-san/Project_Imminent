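; StartGame_BP is a clickable menu actor that starts the game.
; Hovering the cursor over its Box toggles a SpotLight on and off as highlight feedback.
; Clicking it plays the GameStart level sequence, waits for the sequence's length, then opens the P_Cave level.
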(event OnBeginCursorOver(Box)
  (params (TouchedComponent :type Primitive%20Component%20Object%20Reference))
  (Rendering|SetVisibility (Variables|Default|GetSpotLight) true false))

(event OnEndCursorOver(Box)
  (params (TouchedComponent :type Primitive%20Component%20Object%20Reference))
  (Rendering|SetVisibility (Variables|Default|GetSpotLight) false false))

(event EventBeginPlay)

(event EventTick
  (params (DeltaSeconds :type Float%20%28single-precision%29)))

(event MouseInput|EventActorOnClicked
  (params (ButtonPressed :type Key%20Structure :default "AnyKey"))
  (bind _returnvalue (Sequencer|Player|CreateLevelSequencePlayer "/Game/ImminentCPP/Menu/GameStart.GameStart"))
  (Audio|Components|Audio|Play _returnvalue)
  (Utilities|FlowControl|Delay (Class|LevelSequencePlayer|GetLength _returnvalue))
  (Game|OpenLevel(byName) "P_Cave"))

(fn ConstructionScript)